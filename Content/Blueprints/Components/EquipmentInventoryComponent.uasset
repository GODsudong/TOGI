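; Inventory component subclass that adds character equipment slots, reserving the first inventory indices for the equipment slot enum entries.
; Init and load enlarge the inventory by that count, and the empty-space search skips those slots.
; Set and clear overrides refresh equipped visuals: armor slots assign character meshes, while hand slots respawn socket-attached actors.
; Hand spawning casts specifically to the one-hand sword and wooden shield classes; back and belt assignments are unconnected.
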(event EventBeginPlay)

(event EventTick
  (params (DeltaSeconds :type Float%20%28single-precision%29)))

(fn GetEmptyInventorySpace
  (for (_array_element _array_index) (Variables|Default|GetInventory)
    (if (not (Utilities|IsValid (.Icon (Utilities|Struct|BreakItemDatainfo _array_element)))) ; Is It Empty?
      (if (>= _array_index (|GetNumEnumEntries)) ; Do not Return Equipment Slots
        (LocalVariables|SetLocalIndex _array_index)
        (LocalVariables|SetLocalSuccess true))))
  (return (LocalVariables|GetLocalSuccess) (LocalVariables|GetLocalIndex)))

(fn SetInventoryItem
  (params (InventorySlot :type Integer) (InventoryItem :type Item%20Datainfo%20Structure))
  (bind _success (|CallParentFunction InventorySlot InventoryItem))
  (CallFunction|UpdateEquippedMeshes InventorySlot)
  (return _success))

(fn UpdateEquippedMeshes
  (params (Inventory%20Slot :type Integer))
  (bind _characterreference (Variables|Default|GetCharacterReference))
  (bind _characterreference_2 (Variables|Default|GetCharacterReference))
  (Utilities|IsValid (Variables|Default|GetCharacterReference)
    (:Is%20Valid
      (if (< Inventory%20Slot (|GetNumEnumEntries))
        (bind _inventoryitem (CallFunction|GetInventoryItem Inventory%20Slot))
        (LocalVariables|SetLocalEquipmentMesh (.EquipmentMesh (Utilities|Struct|BreakItemDatainfo _inventoryitem)))
        (LocalVariables|SetLocalWeaponMesh (.WeaponMesh (Utilities|Struct|BreakItemDatainfo _inventoryitem)))
        (LocalVariables|SetLocalWeaponActorClass (.WeaponActorClass (Utilities|Struct|BreakItemDatainfo _inventoryitem)))
        (switch Utilities|FlowControl|Switch|SwitchonEquipmentSlots (Utilities|Enum|ByteToEnumEquipmentSlots (Math|Conversions|ToByte(Integer) Inventory%20Slot))
          (:NewEnumerator0
            (Variables|/Game/Blueprints/Character/BP_MyPlayer.BP_MyPlayer_C|SetHeadMesh _characterreference (LocalVariables|GetLocalEquipmentMesh)))
          (:NewEnumerator1
            (Variables|/Game/Blueprints/Character/BP_MyPlayer.BP_MyPlayer_C|SetBodyMesh _characterreference (LocalVariables|GetLocalEquipmentMesh)))
          (:NewEnumerator2
            (Variables|/Game/Blueprints/Character/BP_MyPlayer.BP_MyPlayer_C|SetGlovesMesh _characterreference (LocalVariables|GetLocalEquipmentMesh)))
          (:NewEnumerator3
            (Variables|/Game/Blueprints/Character/BP_MyPlayer.BP_MyPlayer_C|SetShoesMesh _characterreference (LocalVariables|GetLocalEquipmentMesh)))
          (:NewEnumerator4
            (CallFunction|UpdateLeftHandWeapon (LocalVariables|GetLocalWeaponActorClass))
            (Default|CanShieldGuard _characterreference_2))
          (:NewEnumerator5
            (CallFunction|UpdateRightHandWeapon (LocalVariables|GetLocalWeaponActorClass))
            (Default|CanWeaponAttack _characterreference_2)))))))

(fn LoadInventoryItems
  (params (InventorySize :type Integer) (InventoryItems :type Array%20of%20Item%20Datainfo%20Structures))
  (bind _success (|CallParentFunction (+ (|GetNumEnumEntries) InventorySize) InventoryItems))
  (return _success))

(fn ClearInventoryItem
  (params (InventorySlot :type Integer))
  (bind _success (|CallParentFunction InventorySlot))
  (CallFunction|UpdateEquippedMeshes InventorySlot)
  (return _success))

(fn InitInventory
  (params (InventorySize :type Integer))
  (Utilities|Array|Clear (Variables|Default|GetInventory))
  (for _index (range 0 (+ (|GetNumEnumEntries) (- InventorySize 1)))
    (Utilities|Array|Add :TargetArray (Variables|Default|GetInventory)))
  (return false))

(fn UpdateRightHandWeapon
  (params (WeaponClass :type Object%20Class%20Reference))
  (bind _characterreference (Variables|Default|GetCharacterReference))
  (LocalVariables|SetLocalWeaponActorClass WeaponClass)
  (if (Utilities|IsValid (Variables|/Game/Blueprints/Character/BP_MyPlayer.BP_MyPlayer_C|GetWeaponReference (Variables|Default|GetCharacterReference)))
    (Actor|DestroyActor (Variables|/Game/Blueprints/Character/BP_MyPlayer.BP_MyPlayer_C|GetWeaponReference (Variables|Default|GetCharacterReference)))
    (Variables|/Game/Blueprints/Character/BP_MyPlayer.BP_MyPlayer_C|SetWeaponReference (Variables|Default|GetCharacterReference) 0))
  (if (Utilities|IsValidClass (LocalVariables|GetLocalWeaponActorClass))
    (bind _asbp_weapon_one_hand_sword (Utilities|Casting|CastToBP_Weapon_One_Hand_SwordClass (LocalVariables|GetLocalWeaponActorClass)))
    (bind _returnvalue (Game|SpawnActorfromClass _asbp_weapon_one_hand_sword (Math|Transform|MakeTransform "0, 0, 0" "0, 0, 0" "1,1,1") "Undefined" 0 _characterreference 0))
    (bind _output_get (Variables|/Game/Blueprints/Character/BP_MyPlayer.BP_MyPlayer_C|SetWeaponReference _characterreference _returnvalue))
    (Transformation|AttachComponentToComponent _output_get (Variables|/Script/Engine.Character|GetMesh _characterreference) "RightWeaponShield" "KeepRelative" "KeepRelative" "KeepRelative" true)))

(fn UpdateLeftHandWeapon
  (params (WeaponClass :type Object%20Class%20Reference))
  (bind _characterreference (Variables|Default|GetCharacterReference))
  (LocalVariables|SetLocalWeaponActorClass WeaponClass)
  (if (Utilities|IsValid (Variables|/Game/Blueprints/Character/BP_MyPlayer.BP_MyPlayer_C|GetShieldReference (Variables|Default|GetCharacterReference)))
    (Actor|DestroyActor (Variables|/Game/Blueprints/Character/BP_MyPlayer.BP_MyPlayer_C|GetShieldReference (Variables|Default|GetCharacterReference)))
    (Variables|/Game/Blueprints/Character/BP_MyPlayer.BP_MyPlayer_C|SetShieldReference (Variables|Default|GetCharacterReference) 0))
  (if (Utilities|IsValidClass (LocalVariables|GetLocalWeaponActorClass))
    (bind _asbp_weapon_wooden_shield (Utilities|Casting|CastToBP_Weapon_Wooden_ShieldClass (LocalVariables|GetLocalWeaponActorClass)))
    (bind _returnvalue (Game|SpawnActorfromClass _asbp_weapon_wooden_shield (Math|Transform|MakeTransform "0, 0, 0" "0, 0, 0" "1,1,1") "Undefined" _characterreference _characterreference 0))
    (bind _output_get (Variables|/Game/Blueprints/Character/BP_MyPlayer.BP_MyPlayer_C|SetShieldReference _characterreference _returnvalue))
    (Transformation|AttachComponentToComponent _output_get (Variables|/Script/Engine.Character|GetMesh _characterreference) "LeftWeaponShield" "KeepRelative" "KeepRelative" "KeepRelative" true)))