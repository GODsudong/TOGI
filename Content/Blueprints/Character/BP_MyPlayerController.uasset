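; Player controller that owns the player's stats, health, weapon damage, shield guard and inventory input, quitting the game at zero health.
; Startup links character, HUD and inventory components, then loads a Knight loadout from data tables.
; UI events forward to InventoryManagerComponent; equip, unequip and use rebuild stats from equipment bonuses plus base values, also refilling health.
; Holding Ability with a shield slows movement, enables shield collision and opens a brief SuperGuard window.
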(event Custom|Weapon%20Attack
  (params (Monster :type Actor%20Object%20Reference))
  (Game|Damage|ApplyDamage Monster (.Damage (Utilities|Struct|BreakStatusPoint (Variables|Default|GetPlayerStatus))) 0 (Variables|Default|GetCharacter%20Reference) "/Game/Blueprints/Character/DamageType_WeaponAttack.DamageType_WeaponAttack_C")
  (Audio|PlaySoundatLocation "/Game/Sound/SFX/MagicSkills/5MedievalWeapons/Dagga_01/Cue/Sword_Hit_Sound.Sword_Hit_Sound" (Transformation|GetActorLocation (Variables|Default|GetCharacter%20Reference)) "0, 0, 0" 1.0 1.0 0.0 0 0 0))

(event Custom|UI_Close_Inventory
  ;[1 1 1] UI 이벤트
  ;;[1 1 1] 코멘트
  (Default|ClientCloseInventory (Variables|Default|GetInventoryManagerComponent)))

(event Custom|UI_Split_Inventory_Item
  (params (FromInventorySlot :type Integer) (ToInventorySlot :type Integer) (Amount :type Integer))
  ;[1 1 1] UI 이벤트
  ;;[1 1 1] 코멘트
  (Default|ServerSplitInventoryItem (Variables|Default|GetInventoryManagerComponent) FromInventorySlot ToInventorySlot Amount))

(event Custom|UI_Drop_Inventory_Item
  (params (FromInventorySlot :type Integer))
  ;[1 1 1] UI 이벤트
  ;;[1 1 1] 코멘트
  (Default|ServerDropItemfromInventory (Variables|Default|GetInventoryManagerComponent) FromInventorySlot))

(event Custom|DamageEvent
  (params (Damage :type Float%20%28single-precision%29))
  (bind _output_get (Variables|Default|SetHealth (- (Variables|Default|GetHealth) (- Damage (.Defense (Utilities|Struct|BreakStatusPoint (Variables|Default|GetPlayerStatus)))))))
  (if (<= _output_get 0.0)
    (Game|QuitGame 0 "Quit" false)))

(event Custom|UI_Set_Is_Mouse_Over_UI
  (params (IsMouseOverUI :type Boolean))
  ;[1 1 1] UI 이벤트
  ;;[1 1 1] 코멘트
  (Variables|입력|SetIsMouseOverUI IsMouseOverUI))

(event Custom|UI_Use_Inventory_Item
  (params (InventorySlot :type Integer))
  ;[1 1 1] UI 이벤트
  ;;[1 1 1] 코멘트
  (Default|ServerUseInventoryItem (Variables|Default|GetInventoryManagerComponent) InventorySlot)
  (CallFunction|UpdatePlayertStats))

(event Custom|UI_Equip_Inventory_Item
  (params (FromInventorySlot :type Integer) (ToInventorySlot :type Integer))
  ;[1 1 1] UI 이벤트
  ;;[1 1 1] 코멘트
  (Default|ServerEquipfromInventory (Variables|Default|GetInventoryManagerComponent) FromInventorySlot ToInventorySlot)
  (CallFunction|UpdatePlayertStats))

(event Custom|UI_Un_Equip_Inventory_Item
  (params (FromInventorySlot :type Integer) (ToInventorySlot :type Integer))
  ;[1 1 1] UI 이벤트
  ;;[1 1 1] 코멘트
  (Default|ServerUnequiptoInventory (Variables|Default|GetInventoryManagerComponent) FromInventorySlot ToInventorySlot)
  (CallFunction|UpdatePlayertStats))

(event Custom|UI_Move_Inventory_Item
  (params (FromInventorySlot :type Integer) (ToInventorySlot :type Integer))
  ;[1 1 1] UI 이벤트
  ;;[1 1 1] 코멘트
  (Default|ServerMoveInventoryItem (Variables|Default|GetInventoryManagerComponent) FromInventorySlot ToInventorySlot))

(event EventBeginPlay
  (Input|DisableInput 0)
  (Utilities|FlowControl|Delay 1.0)
  (CallFunction|InitializePlayer)
  (Input|EnableInput 0))

(event Input|ActionEvents|InputActionAbility
  (params (Key :type Key%20Structure :default "None"))
  (bind _playerstatus (Variables|Default|GetPlayerStatus))
  (bind _character_reference (Variables|Default|GetCharacter%20Reference))
  (bind _character_reference_2 (Variables|Default|GetCharacter%20Reference))
  (bind _movementspeed (Utilities|Struct|BreakStatusPoint _playerstatus))
  (bind _shieldreference (Variables|/Game/Blueprints/Character/BP_MyPlayer.BP_MyPlayer_C|GetShieldReference _character_reference))
  (bind _charactermovement (Variables|/Script/Engine.Character|GetCharacterMovement _character_reference))
  (bind _isshieldequipped (Variables|/Game/Blueprints/Character/BP_MyPlayer.BP_MyPlayer_C|GetIsShieldEquipped _character_reference_2))
  (bind _box (Variables|/Game/Blueprints/Character/BP_Weapon.BP_Weapon_C|GetBox _shieldreference))
  (:Pressed
    (if _isshieldequipped
      (Variables|Default|SetPreesed true)
      (Utilities|FlowControl|Delay 0.2)
      (if (Variables|Default|GetPreesed)
        (Utilities|FlowControl|Sequence
          (:then_0
            (Variables|Default|SetGuard true)
            (Variables|/Script/Engine.CharacterMovementComponent|SetMaxWalkSpeed _charactermovement (/ _movementspeed 3.0))
            (Collision|SetCollisionEnabled _box "QueryOnly"))
          (:then_1
            (Variables|Default|SetSuperGuard true)
            (Utilities|FlowControl|Delay 0.2)
            (Variables|Default|SetSuperGuard false))))))
  (:Released
    (if _isshieldequipped
      (Variables|Default|SetPreesed false)
      (Variables|Default|SetGuard false)
      (Variables|/Script/Engine.CharacterMovementComponent|SetMaxWalkSpeed _charactermovement _movementspeed)
      (Collision|SetCollisionEnabled _box "NoCollision"))))

(event Input|ActionEvents|InputActionStatus
  (params (Key :type Key%20Structure :default "None"))
  (bind _inventorymanagercomponent (Variables|Default|GetInventoryManagerComponent))
  ;[1 1 1] 인풋 이벤트
  (:Pressed
    (if (Variables|/Game/Blueprints/Components/InventoryManagerComponent.InventoryManagerComponent_C|GetIsInventoryOpen (Variables|Default|GetInventoryManagerComponent))
      (Default|ClientCloseInventory _inventorymanagercomponent)
      (Default|ClientCloseEquipment _inventorymanagercomponent)
      (Variables|Default|SetbShowMouseCursor false)
      (else
        (Default|ClientOpenInventory _inventorymanagercomponent)
        (Default|ClientOpenEquipment _inventorymanagercomponent)
        (Variables|Default|SetbShowMouseCursor true)))))

(event Input|MouseEvents|RightMouseButton
  (params (Key :type Key%20Structure :default "None"))
  ;[1 1 1] 인풋 이벤트
  (:Pressed
    (Variables|입력|SetIsRightMouseButtonDown true))
  (:Released
    (Variables|입력|SetIsRightMouseButtonDown false)))

(event Input|KeyboardEvents|RightBracket
  (params (Key :type Key%20Structure :default "None"))
  ;[1 1 1] 인풋 이벤트
  (:Pressed
    (Default|ServerIncreaseInventorySize (Variables|Default|GetInventoryManagerComponent) 1)))

(event Input|KeyboardEvents|LeftBracket
  (params (Key :type Key%20Structure :default "None"))
  ;[1 1 1] 인풋 이벤트
  (:Pressed
    (Default|ServerDecreaseInventorySize (Variables|Default|GetInventoryManagerComponent) 1)))

(fn ConstructionScript)

(fn InitializePlayer
  (bind _equipmentinventorycomponent (Variables|Default|GetEquipmentInventoryComponent))
  (bind _asbp_my_player (Utilities|Casting|CastToBP_MyPlayer (Pawn|GetControlledPawn)))
  (bind _output_get (Variables|Default|SetCharacter%20Reference _asbp_my_player))
  (Variables|/Game/Blueprints/Components/EquipmentInventoryComponent.EquipmentInventoryComponent_C|SetCharacterReference _equipmentinventorycomponent _output_get)
  (Default|InitializeInventoryManger (Variables|Default|GetInventoryManagerComponent) _equipmentinventorycomponent)
  (CallFunction|ServerLoadPlayerItems)
  (bind _asbp_my_player_hud (Utilities|Casting|CastToBP_MyPlayerHUD (HUD|GetHUD)))
  (bind _output_get_2 (Variables|Default|SetHUDReference (Variables|/Game/Blueprints/Character/BP_MyPlayerHUD.BP_MyPlayerHUD_C|GetHUDReference _asbp_my_player_hud)))
  (Default|InitializeStatusUI (Variables|Default|GetInventoryManagerComponent) (Variables|/Game/UI/Blueprint/BP_CharacterHUD.BP_CharacterHUD_C|GetBP_StatusUI _output_get_2))
  (Default|ClientLoadInventory (Variables|Default|GetInventoryManagerComponent))
  (CallFunction|UpdatePlayertStats))

(fn ServerLoadPlayerItems
  (bind _localinventory (LocalVariables|GetLocalInventory))
  (bind _returnvalue (Utilities|GetDataTableRow "/Game/Blueprints/Character/StartingInventory.StartingInventory" "Knight")
    (:then
      (bind _output_get (LocalVariables|SetLocalItemIDs (Utilities|Array|MakeArray (.Head (Utilities|Struct|BreakStartingSturct _returnvalue)) (.Body (Utilities|Struct|BreakStartingSturct _returnvalue)) (.Gloves (Utilities|Struct|BreakStartingSturct _returnvalue)) (.Shoes (Utilities|Struct|BreakStartingSturct _returnvalue)) (.LeftHand (Utilities|Struct|BreakStartingSturct _returnvalue)) (.RightHand (Utilities|Struct|BreakStartingSturct _returnvalue)) (.Accessory1 (Utilities|Struct|BreakStartingSturct _returnvalue)) (.Accessory2 (Utilities|Struct|BreakStartingSturct _returnvalue)))))
      (for (_array_element _array_index) _output_get
        (bind _returnvalue_2 (Utilities|GetDataTableRow "/Game/Items/Itemlist_0_3V.Itemlist_0_3V" _array_element)
          (:then
            (Utilities|Array|SetArrayElem _localinventory _array_index _returnvalue_2 true))
          (:RowNotFound
            (Utilities|Array|SetArrayElem :TargetArray _localinventory :Index _array_index :bSizeToFit true))))
      (for _array_element_2 (.Inventory (Utilities|Struct|BreakStartingSturct _returnvalue))
        (bind _returnvalue_3 (Utilities|GetDataTableRow "/Game/Items/Itemlist_0_3V.Itemlist_0_3V" (.ID (Utilities|Struct|BreakItems _array_element_2)))
          (:then
            (bind _structout (Utilities|Struct|SetmembersinItemDatainfo _returnvalue_3 (.Amount (Utilities|Struct|BreakItems _array_element_2))))
            (Utilities|Array|Add (LocalVariables|GetLocalInventory) _structout))))
      (Default|LoadInventoryItems (Variables|Default|GetEquipmentInventoryComponent) (Variables|/Game/Blueprints/Components/InventoryManagerComponent.InventoryManagerComponent_C|GetInventorySize (Variables|Default|GetInventoryManagerComponent)) (LocalVariables|GetLocalInventory)))))

(fn GetPlayerStats
  (return (Variables|Default|GetPlayerStatus)))

(fn UpdatePlayertStats
  (bind _inventorymanagercomponent (Variables|Default|GetInventoryManagerComponent))
  (bind _equipmentstatuspoint (Variables|/Game/Blueprints/Components/InventoryManagerComponent.InventoryManagerComponent_C|GetEquipmentStatusPoint _inventorymanagercomponent))
  (bind (_maxhp _maxhppercent _damage _defense _movementspeed _maxstamina _regenstamina _criticalchance _cooldown _attackdelay) (Utilities|Struct|BreakStatusPoint _equipmentstatuspoint))
  (bind _structout (Utilities|Struct|SetmembersinStatusPoint (Variables|Default|GetPlayerStatus) (* (+ _maxhp 1e+02) _maxhppercent) _maxhppercent (+ _damage 0.0) (+ _defense 0.0) (+ _movementspeed 4e+02) (+ _maxstamina 1e+02) (+ _regenstamina 1e+01) (+ _criticalchance 0.0) (+ _cooldown 0.0) (+ _attackdelay 0.0)))
  (bind _output_get (Variables|Default|SetPlayerStatus _structout))
  (Variables|/Script/Engine.CharacterMovementComponent|SetMaxWalkSpeed (Variables|/Script/Engine.Character|GetCharacterMovement (Variables|Default|GetCharacter%20Reference)) (.MovementSpeed (Utilities|Struct|BreakStatusPoint _output_get)))
  (Variables|Default|SetHealth (.MaxHp (Utilities|Struct|BreakStatusPoint _output_get))))

(fn GetToolTipInfo
  (params (Item%20ID :type Name))
  (bind _returnvalue (Utilities|GetDataTableRow "/Game/Items/Itemlist_0_3V.Itemlist_0_3V" Item%20ID)
    (:then
      _)
    (:RowNotFound
      _))
  (return _returnvalue))