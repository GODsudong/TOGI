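; Player character with modular, replicated equipment visuals that forwards damage taken to its cached BP_MyPlayerController.
; RepNotify functions swap helmet, body, gloves, shoes, belt and back meshes, with default meshes for empty body, glove and shoe slots.
; Skeletal parts follow the main Mesh through master pose; the helmet notify reads HeadMesh, while HeadMesh's own notify is empty.
; Helper functions set weapon and shield equipped flags from reference validity.
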(event Game|Damage|EventAnyDamage
  (params (Damage :type Float%20%28single-precision%29) (DamageType :type Damage%20Type%20Object%20Reference) (InstigatedBy :type Controller%20Object%20Reference) (DamageCauser :type Actor%20Object%20Reference))
  (Default|DamageEvent (Variables|Default|GetControllerReference) Damage))

(event EventBeginPlay
  (bind _asbp_my_player_controller (Utilities|Casting|CastToBP_MyPlayerController (Pawn|GetController)))
  (Variables|Default|SetControllerReference _asbp_my_player_controller))

(fn ConstructionScript
  (Class|SkinnedMeshComponent|SetMasterPoseComponent (Variables|Default|GetFace) (Variables|Character|GetMesh) false))

(fn OnRepHelmetMesh
  (Class|SkinnedMeshComponent|SetSkeletalMesh (Variables|Default|GetHelmet) (Variables|Equipment|GetHeadMesh) true)
  (Class|SkinnedMeshComponent|SetMasterPoseComponent (Variables|Default|GetHelmet) (Variables|Character|GetMesh) false))

(fn OnRepBodyMesh
  (bind _mesh (Variables|Character|GetMesh))
  (bind _bodymesh (Variables|Equipment|GetBodyMesh))
  (Utilities|IsValid _bodymesh
    (:Is%20Valid
      (Class|SkinnedMeshComponent|SetSkeletalMesh _mesh _bodymesh true))
    (:Is%20Not%20Valid
      (Class|SkinnedMeshComponent|SetSkeletalMesh _mesh "/Game/Character/Meshes/ModularBodyParts/Cloth02SK.Cloth02SK" true))))

(fn OnRepGlovesMesh
  (bind _gloves (Variables|Default|GetGloves))
  (bind _glovesmesh (Variables|Equipment|GetGlovesMesh))
  (Utilities|IsValid _glovesmesh
    (:Is%20Valid
      (Class|SkinnedMeshComponent|SetSkeletalMesh _gloves _glovesmesh true))
    (:Is%20Not%20Valid
      (Class|SkinnedMeshComponent|SetSkeletalMesh _gloves "/Game/Character/Meshes/ModularBodyParts/Glove01SK.Glove01SK" true)))
  (Class|SkinnedMeshComponent|SetMasterPoseComponent (Variables|Default|GetGloves) (Variables|Character|GetMesh) false))

(fn OnRepShoesMesh
  (bind _shoes (Variables|Default|GetShoes))
  (bind _shoesmesh (Variables|Equipment|GetShoesMesh))
  (Utilities|IsValid _shoesmesh
    (:Is%20Valid
      (Class|SkinnedMeshComponent|SetSkeletalMesh _shoes _shoesmesh true))
    (:Is%20Not%20Valid
      (Class|SkinnedMeshComponent|SetSkeletalMesh _shoes "/Game/Character/Meshes/ModularBodyParts/Shoe01SK.Shoe01SK" true)))
  (Class|SkinnedMeshComponent|SetMasterPoseComponent (Variables|Default|GetShoes) (Variables|Character|GetMesh) false))

(fn OnRepBeltMesh
  (Class|SkinnedMeshComponent|SetSkeletalMesh (Variables|Default|GetBelt) (Variables|Equipment|GetBeltMesh) true)
  (Class|SkinnedMeshComponent|SetMasterPoseComponent (Variables|Default|GetBelt) (Variables|Character|GetMesh) false))

(fn OnRepBackMesh
  (Components|StaticMesh|SetStaticMesh (Variables|Default|GetBack) (Variables|Equipment|GetBackMesh)))

(fn OnRepHeadMesh)

(fn CanWeaponAttack
  (Utilities|IsValid (Variables|Default|GetWeaponReference)
    (:Is%20Valid
      (Variables|Default|SetisEquipped true))
    (:Is%20Not%20Valid
      (Variables|Default|SetisEquipped false))))

(fn CanShieldGuard
  (Utilities|IsValid (Variables|Default|GetShieldReference)
    (:Is%20Valid
      (Variables|Default|SetIsShieldEquipped true))
    (:Is%20Not%20Valid
      (Variables|Default|SetIsShieldEquipped false))))