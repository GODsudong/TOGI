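; One-handed sword weapon Blueprint that reports hits to the player controller when its Box collision begins an overlap.
; The overlap casts the controller from CharacterReferences to BP_MyPlayerController and calls WeaponAttack with the overlapped actor.
; It stores the first hit as HittedMonster and, while that stays valid, skips repeat overlaps with it but attacks other actors without updating it.
; Tick and the construction script only call their parents.
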(event OnComponentBeginOverlap(Box)
  (params (OverlappedComponent :type Primitive%20Component%20Object%20Reference) (OtherActor :type Actor%20Object%20Reference) (OtherComp :type Primitive%20Component%20Object%20Reference) (OtherBodyIndex :type Integer) (bFromSweep :type Boolean) (SweepResult :type Hit%20Result%20Structure%20%28by%20ref%29))
  (bind _asbp_my_player_controller (Utilities|Casting|CastToBP_MyPlayerController (Pawn|GetController (Variables|Default|GetCharacterReferences))))
  (Utilities|IsValid (Variables|Default|GetHittedMonster)
    (:Is%20Valid
      (bind _output_get (Variables|Default|SetNewMonster OtherActor))
      (if (not (== _output_get (Variables|Default|GetHittedMonster)))
        (Default|WeaponAttack _asbp_my_player_controller _output_get)))
    (:Is%20Not%20Valid
      (Variables|Default|SetHittedMonster OtherActor)
      (Default|WeaponAttack _asbp_my_player_controller OtherActor))))

(event EventTick
  (params (DeltaSeconds :type Float%20%28single-precision%29))
  (|CallParentFunction DeltaSeconds))

(fn ConstructionScript
  (|CallParentFunction))